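; DoorTeleport_BP is an actor with two doors that teleports the player between them.
; On BeginPlay it caches both door world locations, with debug prints.
; Overlapping either collider calls a function that moves the first BP_PersoPrincipal actor to the other door plus a fixed offset, briefly toggling player input around the move.
; The overlap events do not check which actor entered.
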(event OnComponentBeginOverlap(collide)
  (params (OverlappedComponent :type Primitive%20Component%20Object%20Reference) (OtherActor :type Actor%20Object%20Reference) (OtherComp :type Primitive%20Component%20Object%20Reference) (OtherBodyIndex :type Integer) (bFromSweep :type Boolean) (SweepResult :type Hit%20Result%20Structure%20%28by%20ref%29))
  (bind _returnvalue (Game|GetPlayerCharacter 0))
  (bind _returnvalue_2 (Game|GetPlayerController 0))
  ;[1 1 1] Teleport between 2 Doors
  (Input|DisableInput _returnvalue _returnvalue_2)
  (CallFunction|Teleport1/2)
  (Input|EnableInput _returnvalue _returnvalue_2))

(event OnComponentBeginOverlap(collide2)
  (params (OverlappedComponent :type Primitive%20Component%20Object%20Reference) (OtherActor :type Actor%20Object%20Reference) (OtherComp :type Primitive%20Component%20Object%20Reference) (OtherBodyIndex :type Integer) (bFromSweep :type Boolean) (SweepResult :type Hit%20Result%20Structure%20%28by%20ref%29))
  (bind _returnvalue (Game|GetPlayerCharacter 0))
  (bind _returnvalue_2 (Game|GetPlayerController 0))
  ;[1 1 1] Teleport between 2 Doors
  (Input|DisableInput _returnvalue _returnvalue_2)
  (CallFunction|Teleport2/1)
  (Input|EnableInput _returnvalue _returnvalue_2))

(event EventBeginPlay
  ;[1 1 1] All the variables
  (bind _output_get (Variables|Default|SetLocationDoor1 (Transformation|GetWorldLocation (Variables|Default|GetDoor))))
  (Development|PrintString (Utilities|String|Append "Porte 1: " (Utilities|String|ToString(Vector) _output_get)) true true "(R=0.000000,G=0.660000,B=1.000000,A=1.000000)" 6e+01)
  (bind _output_get_2 (Variables|Default|SetLocationDoor2 (Transformation|GetWorldLocation (Variables|Default|GetDoor2))))
  (Development|PrintString (Utilities|String|Append "Porte 2: " (Utilities|String|ToString(Vector) _output_get_2)) true true "(R=0.095151,G=1.000000,B=0.000000,A=1.000000)" 6e+01))

(fn ConstructionScript)

(fn Teleport1/2
  (bind _outactors (Actor|GetAllActorsOfClass "/Game/Blueprints/BP_PersoPrincipal.BP_PersoPrincipal_C"))
  (Development|PrintString (Utilities|String|ToString(Vector) (Transformation|GetActorLocation (Utilities|Array|Get(acopy) _outactors))) true true "(R=0.000000,G=0.660000,B=1.000000,A=1.000000)" 5.0)
  (Transformation|SetWorldLocation (Variables|/Script/Engine.Actor|GetRootComponent (Utilities|Array|Get(acopy) _outactors)) (+ (Variables|Default|GetLocationDoor2) "-75.000000,-200.000000,0.000000") false false))

(fn Teleport2/1
  (bind _outactors (Actor|GetAllActorsOfClass "/Game/Blueprints/BP_PersoPrincipal.BP_PersoPrincipal_C"))
  (Development|PrintString (Utilities|String|ToString(Vector) (Transformation|GetActorLocation (Utilities|Array|Get(acopy) _outactors))))
  (Transformation|SetWorldLocation (Variables|/Script/Engine.Actor|GetRootComponent (Utilities|Array|Get(acopy) _outactors)) (+ (Variables|Default|GetLocationDoor1) "-75.000000,200.000000,0.000000") false false))