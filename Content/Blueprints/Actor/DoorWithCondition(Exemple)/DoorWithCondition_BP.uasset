(event OnComponentBeginOverlap(Box1)
  (params (OverlappedComponent :type Primitive%20Component%20Object%20Reference) (OtherActor :type Actor%20Object%20Reference) (OtherComp :type Primitive%20Component%20Object%20Reference) (OtherBodyIndex :type Integer) (bFromSweep :type Boolean) (SweepResult :type Hit%20Result%20Structure%20%28by%20ref%29))
  (bind _outactors (Actor|GetAllActorsOfClass "/Game/Blueprints/BP_PersoPrincipal.BP_PersoPrincipal_C"))
  (if (== (Variables|/Game/Blueprints/BP_PersoPrincipal.BP_PersoPrincipal_C|GetnombreDeCube (Utilities|Array|Get(acopy) _outactors)) 4)
    (CallFunction|Teleport2/1)
    (else
      (bind _returnvalue (UserInterface|CreateWidget "/Game/Blueprints/Actor/DoorWithCondition(Exemple)/Youcant_Widget.Youcant_Widget_C"))
      (UserInterface|Viewport|AddtoViewport _returnvalue 0))))

(event OnComponentBeginOverlap(Box)
  (params (OverlappedComponent :type Primitive%20Component%20Object%20Reference) (OtherActor :type Actor%20Object%20Reference) (OtherComp :type Primitive%20Component%20Object%20Reference) (OtherBodyIndex :type Integer) (bFromSweep :type Boolean) (SweepResult :type Hit%20Result%20Structure%20%28by%20ref%29))
  (bind _outactors (Actor|GetAllActorsOfClass "/Game/Blueprints/BP_PersoPrincipal.BP_PersoPrincipal_C"))
  (if (== (Variables|/Game/Blueprints/BP_PersoPrincipal.BP_PersoPrincipal_C|GetnombreDeCube (Utilities|Array|Get(acopy) _outactors)) 4)
    (CallFunction|Teleport1/2)
    (else
      (bind _returnvalue (UserInterface|CreateWidget "/Game/Blueprints/Actor/DoorWithCondition(Exemple)/Youcant_Widget.Youcant_Widget_C"))
      (UserInterface|Viewport|AddtoViewport _returnvalue 0))))

(event OnComponentEndOverlap(Box)
  (params (OverlappedComponent :type Primitive%20Component%20Object%20Reference) (OtherActor :type Actor%20Object%20Reference) (OtherComp :type Primitive%20Component%20Object%20Reference) (OtherBodyIndex :type Integer))
  (bind _foundwidgets (Widget|GetAllWidgetsOfClass "/Game/Blueprints/Actor/DoorWithCondition(Exemple)/Youcant_Widget.Youcant_Widget_C" true))
  (Widget|RemovefromParent (Utilities|Array|Get(acopy) _foundwidgets)))

(event OnComponentEndOverlap(Box1)
  (params (OverlappedComponent :type Primitive%20Component%20Object%20Reference) (OtherActor :type Actor%20Object%20Reference) (OtherComp :type Primitive%20Component%20Object%20Reference) (OtherBodyIndex :type Integer))
  (bind _foundwidgets (Widget|GetAllWidgetsOfClass "/Game/Blueprints/Actor/DoorWithCondition(Exemple)/Youcant_Widget.Youcant_Widget_C" true))
  (Widget|RemovefromParent (Utilities|Array|Get(acopy) _foundwidgets)))

(event EventBeginPlay
  (bind _output_get (Variables|Default|SetLocationDoor1 (Transformation|GetWorldLocation (Variables|Default|GetStaticMesh))))
  (Development|PrintString (Utilities|String|Append "Porte 1: " (Utilities|String|ToString(Vector) _output_get)) true true "(R=0.000000,G=0.660000,B=1.000000,A=1.000000)" 6e+01)
  (bind _output_get_2 (Variables|Default|SetLocationDoor2 (Transformation|GetWorldLocation (Variables|Default|GetStaticMesh1))))
  (Development|PrintString (Utilities|String|Append "Porte 2: " (Utilities|String|ToString(Vector) _output_get_2)) true true "(R=0.095151,G=1.000000,B=0.000000,A=1.000000)" 6e+01))

(fn ConstructionScript)

(fn Teleport1/2
  (bind _outactors (Actor|GetAllActorsOfClass "/Game/Blueprints/BP_PersoPrincipal.BP_PersoPrincipal_C"))
  (Development|PrintString (Utilities|String|ToString(Vector) (Transformation|GetActorLocation (Utilities|Array|Get(acopy) _outactors))) true true "(R=0.000000,G=0.660000,B=1.000000,A=1.000000)" 5.0)
  (Transformation|SetWorldLocation (Variables|/Script/Engine.Actor|GetRootComponent (Utilities|Array|Get(acopy) _outactors)) (+ (Variables|Default|GetLocationDoor2) "-75.000000,-200.000000,0.000000") false false))

(fn Teleport2/1
  (bind _outactors (Actor|GetAllActorsOfClass "/Game/Blueprints/BP_PersoPrincipal.BP_PersoPrincipal_C"))
  (Development|PrintString (Utilities|String|ToString(Vector) (Transformation|GetActorLocation (Utilities|Array|Get(acopy) _outactors))))
  (Transformation|SetWorldLocation (Variables|/Script/Engine.Actor|GetRootComponent (Utilities|Array|Get(acopy) _outactors)) (+ (Variables|Default|GetLocationDoor1) "-75.000000,200.000000,0.000000") false false))